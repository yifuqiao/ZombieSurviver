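; RapidMoveTo is a Behavior Tree task that moves an enemy's pawn toward the actor stored in the TargetToFollow blackboard key.
; On execute it casts the owner to EnemyController_bp, caching the reference for later runs, then calls AIMoveTo on the controlled pawn with a small acceptance radius.
; It finishes successfully when the move succeeds; a failed move or cast never finishes the task.
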(event EventReceiveExecute
  (params (OwnerActor :type Actor%20Object%20Reference))
  (if (!= (Variables|Default|Getenemy_controller_ref) 0)
    _
    (else
      (bind _asenemy_controller_bp (Utilities|Casting|CastToEnemyController_bp OwnerActor))
      (Variables|Default|Setenemy_controller_ref _asenemy_controller_bp)))
  (AI|AIMoveTo (Pawn|GetControlledPawn (Variables|Default|Getenemy_controller_ref)) "0, 0, 0" (AI|BehaviorTree|GetBlackboardValueasActor (Variables|Default|GetTargetToFollow)) 5e+01 false
    (:OnSuccess
      (AI|BehaviorTree|FinishExecute true))))