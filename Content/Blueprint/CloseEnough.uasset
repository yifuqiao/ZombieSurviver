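; Behavior tree decorator that gates enemy AI on its distance from the blackboard actor it follows.
; It casts the owner to EnemyController_bp, caches it, and measures the straight-line distance from the controlled pawn to the TargetToFollow actor.
; Despite the name CloseEnough, the condition passes when that distance is at or beyond AcceptableDistance, meaning the enemy is not yet inside that radius.
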(fn PerformConditionCheck
  (params (OwnerActor :type Actor%20Object%20Reference))
  (bind _asenemy_controller_bp (Utilities|Casting|CastToEnemyController_bp OwnerActor))
  (Variables|Default|SetEnemyControllerRef _asenemy_controller_bp)
  (return (>= (Math|Vector|VectorLength (- (Transformation|GetActorLocation (AI|BehaviorTree|GetBlackboardValueasActor (Variables|Default|GetTargetToFollow))) (Transformation|GetActorLocation (Pawn|GetControlledPawn (Variables|Default|GetEnemyControllerRef))))) (Variables|Default|GetAcceptableDistance))))