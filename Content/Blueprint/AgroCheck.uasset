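; AgroCheck is an AI Behavior Tree node that detects targets around an enemy and writes them to the Blackboard.
; Each tick, it sphere-traces at the pawn's location, ignoring all Ememy_bp actors, then line-traces to each hit to test visibility.
; A visible hit sets TargetToFollow and TargetLocation, while a blocked one clears only TargetToFollow, so the last hit decides.
; An empty sweep leaves both keys unchanged.
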(event EventTick
  (params (OwnerActor :type Actor%20Object%20Reference) (DeltaSeconds :type Float%20%28single-precision%29))
  (if (!= (Variables|Default|GetEmemyControllerRef) 0)
    _
    (else
      (bind _asenemy_controller_bp (Utilities|Casting|CastToEnemyController_bp OwnerActor))
      (Variables|Default|SetEmemyControllerRef _asenemy_controller_bp)))
  (bind _outactors (Actor|GetAllActorsOfClass "/Game/Blueprint/Ememy_bp.Ememy_bp_C"))
  (Variables|Default|SetMyLocation (Transformation|GetActorLocation (Pawn|GetControlledPawn (Variables|Default|GetEmemyControllerRef))))
  (bind _outhits (Collision|MultiSphereTraceForObjects (Transformation|GetActorLocation (Pawn|GetControlledPawn (Variables|Default|GetEmemyControllerRef))) (+ (Transformation|GetActorLocation (Pawn|GetControlledPawn (Variables|Default|GetEmemyControllerRef))) "0, 0, 0") 0.0 (Variables|Default|GetDesiredObjectTypes) false _outactors "None"))
  (bind _array_element (Utilities|Array|ForEachLoopwithBreak _outhits)
    (:LoopBody
      (bind _outhit (Collision|LineTraceByChannel (Variables|Default|GetMyLocation) (Transformation|GetActorLocation (.HitActor (Collision|BreakHitResult _array_element))) "TraceTypeQuery1" false _outactors "None"))
      (if (== (.HitActor (Collision|BreakHitResult _outhit)) (.HitActor (Collision|BreakHitResult _array_element)))
        (Class|BTFunctionLibrary|SetBlackboardValueasObject (Variables|Default|GetTargetToFollow) (.HitActor (Collision|BreakHitResult _outhit)))
        (AI|BehaviorTree|SetBlackboardValueasVector (Variables|Default|GetTargetLocation) (Transformation|GetActorLocation (.HitActor (Collision|BreakHitResult _outhit))))
        (else
          (Class|BTFunctionLibrary|SetBlackboardValueasObject (Variables|Default|GetTargetToFollow)))))))